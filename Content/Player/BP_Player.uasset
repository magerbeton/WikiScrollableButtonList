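; BP_Player is a player Blueprint that hosts the main UI and test-drives its scrollable button list.
; On BeginPlay it creates WBP_Main, adds it to the viewport, shows the cursor and sets Game and UI input focused on the widget.
; A debug key rebuilds a string array of random integers, sized by the widget's max-value spin box, and passes it to WBPScrollableButtonList to spawn buttons.
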(event EventBeginPlay
  (bind _returnvalue (Game|GetPlayerController 0))
  ;[1 1 1] Creates the main widget and sets the input mode accordingly. It shows the mouse cursor
  (bind _returnvalue_2 (UserInterface|CreateWidget "/Game/UI/WBP_Main.WBP_Main_C"))
  (Variables|Default|SetWidgetReference _returnvalue_2)
  (UserInterface|Viewport|AddtoViewport _returnvalue_2 0)
  (Variables|/Script/Engine.PlayerController|SetbShowMouseCursor _returnvalue true)
  (Input|SetInputModeGameandUI _returnvalue _returnvalue_2 "DoNotLock" true false))

(event Input|KeyboardEvents|DebugKey1
  (params (Key :type Key%20Structure :default "None") (ActionValue :type Input%20Action%20Value%20Structure))
  ;[1 1 1] Spawn buttons with dummy data (in this case its random integers. The buttons print foo if the assigned number is uneven and bar if its even)
  (:Pressed
    (Development|PrintString "One Pressed")
    (Utilities|Array|Clear (Variables|Default|GetDynamicStringArray))
    (for _index (range 0 (Math|Float|Truncate (Class|SpinBox|GetValue (Variables|/Game/UI/WBP_Main.WBP_Main_C|GetSpinBox_MaxValue (Variables|Default|GetWidgetReference)))))
      (Utilities|Array|Add (Variables|Default|GetDynamicStringArray) (Utilities|String|ToString(Integer) (Math|Random|RandomIntegerinRange 0 255))))
    (Default|SpawnButtons (Variables|/Game/UI/WBP_Main.WBP_Main_C|GetWBP_ScrollableButtonList (Variables|Default|GetWidgetReference)) (Variables|Default|GetDynamicStringArray))))

(fn ConstructionScript)